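; AI controller for the elephant that runs the BT_Elephant behavior tree on BeginPlay.
; Unconnected graph logic would write a sight target and the average position of itself and perceived elephants to the Blackboard, with a debug sphere.
; Flocking-style helpers are unfinished: CalculateSpeedDifference computes a scaled velocity difference to another elephant, while the average-position and avoidance functions are empty, as is Tick.
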(event EventBeginPlay
  (AI|RunBehaviorTree "/Game/Animals/Elephant/BT_Elephant.BT_Elephant"))

(event EventTick
  (params (DeltaSeconds :type Float%20%28single-precision%29))
  ;[1 1 1] Average Position
)

(fn ConstructionScript)

(fn CalculateAveragePosition
  (params (TargetArray :type Array%20of%20Actor%20Object%20References) (OtherElephant :type Actor%20Object%20Reference)))

(fn CalculateSpeedDifference
  (params (Other%20Elephant :type Actor%20Object%20Reference) (TargetArray :type Array%20of%20BP%20Elephant%20Object%20References))
  (bind _asbp_elephant (Utilities|Casting|CastToBP_Elephant (Pawn|GetControlledPawn self)))
  (Variables|Default|SetSpeedDifference (/ (- (Transformation|GetVelocity Other%20Elephant) (Transformation|GetVelocity _asbp_elephant)) (Utilities|Array|Length TargetArray))))

(fn CalculateAvoidanceVector
  (params (self2 :type Actor%20Object%20Reference) (TargetArray :type Array%20of%20BP%20Elephant%20Object%20References)))